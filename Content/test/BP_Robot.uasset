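; BP_Robot is a test robot Blueprint that moves a Cube component and probes with a debug line trace.
; Events 108 and 110 lower and raise an X step, while event 109 grows a Z step and adds both to the cube's position.
; Event 109 then traces on Visibility to an end point computed by dividing location by offset forward vector, plus NewVar0, and prints hit distance and actor.
; Tick and the construction script are empty.
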(event `108`
  (bind _output_get (set `self.NewVar_3` (- (`self.NewVar_3`) 10)))
  (`KismetSystemLibrary.PrintString` (`KismetStringLibrary.Conv_IntToString` _output_get)))

(event `110`
  (bind _output_get (set `self.NewVar_3` (+ (`self.NewVar_3`) 10)))
  (`KismetSystemLibrary.PrintString` (`KismetStringLibrary.Conv_IntToString` _output_get)))

(event `109`
  (bind _cube (`self.Cube`))
  (bind _cube_2 (`self.Cube`))
  (bind _returnvalue (`SceneComponent.K2_GetComponentLocation` _cube))
  (bind (_returnvalue_x _returnvalue_y _returnvalue_z) (`KismetMathLibrary.BreakVector` (`SceneComponent.K2_GetComponentLocation` _cube_2)))
  (set `self.NewVar_1` (+ (`self.NewVar_1`) 10))
  (`SceneComponent.K2_SetWorldLocation` _cube_2 (`KismetMathLibrary.MakeVector` (+ _returnvalue_x (`KismetMathLibrary.Conv_IntToDouble` (`self.NewVar_3`))) _returnvalue_y (+ _returnvalue_z (`KismetMathLibrary.Conv_IntToDouble` (`self.NewVar_1`)))) false false)
  (`KismetSystemLibrary.PrintString` (`KismetStringLibrary.Conv_IntToString` (`self.NewVar_1`)))
  (bind _outhit (`KismetSystemLibrary.LineTraceSingle` :`Start` _returnvalue :`End` (+ (/ _returnvalue (+ (`SceneComponent.GetForwardVector` _cube) 500)) (`self.NewVar_0`)) :`TraceChannel` "TraceTypeQuery1" :`DrawDebugType` "ForDuration"))
  (bind (_bblockinghit _binitialoverlap _time _distance _location _impactpoint _normal _impactnormal _physmat _hitactor) (`GameplayStatics.BreakHitResult` _outhit))
  (`KismetSystemLibrary.PrintString` (`KismetStringLibrary.Conv_DoubleToString` _distance))
  (`KismetSystemLibrary.PrintString` (`KismetSystemLibrary.GetObjectName` _hitactor)))

(event `Key|Q`
  (params (Key :type "Key Structure")))

(event `self.ReceiveTick`
  (params (DeltaSeconds :type "Float (single-precision)")))

(fn `UserConstructionScript`)